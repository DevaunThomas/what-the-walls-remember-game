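; Key pickup that grants the player a key and triggers a doll scare.
; Overlapping PickupSphere registers it as the first-person character's CurrentKey and shows an interact prompt; leaving clears both.
; Interact sets HasKey, hides HallwayDoll, reveals ScareDoll, plays a whisper at the player and briefly shows a key-found widget before destroying the actor.
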(event `self.PickupSphere.OnComponentBeginOverlap`
  (params (OverlappedComponent :type "PrimitiveComponent Object Reference") (OtherActor :type "Actor Object Reference") (OtherComp :type "PrimitiveComponent Object Reference") (OtherBodyIndex :type Integer) (bFromSweep :type Boolean) (SweepResult :type "HitResult Structure (by ref)"))
  (bind _asbp_first_person_character (cast `/Game/FirstPerson/Blueprints/BP_FirstPersonCharacter` OtherActor))
  (set `/Game/FirstPerson/Blueprints/BP_FirstPersonCharacter.CurrentKey` self _asbp_first_person_character)
  (`/Game/FirstPerson/Blueprints/BP_FirstPersonCharacter.ShowInteractPrompt` _asbp_first_person_character))

(event `self.PickupSphere.OnComponentEndOverlap`
  (params (OverlappedComponent :type "PrimitiveComponent Object Reference") (OtherActor :type "Actor Object Reference") (OtherComp :type "PrimitiveComponent Object Reference") (OtherBodyIndex :type Integer))
  (bind _asbp_first_person_character (cast `/Game/FirstPerson/Blueprints/BP_FirstPersonCharacter` OtherActor))
  (set `/Game/FirstPerson/Blueprints/BP_FirstPersonCharacter.CurrentKey` null _asbp_first_person_character)
  (`/Game/FirstPerson/Blueprints/BP_FirstPersonCharacter.HideInteractPrompt` _asbp_first_person_character))

(event `Interact`
  (bind _asbp_first_person_character (cast `/Game/FirstPerson/Blueprints/BP_FirstPersonCharacter` (`GameplayStatics.GetPlayerCharacter` 0)))
  (set `/Game/FirstPerson/Blueprints/BP_FirstPersonCharacter.HasKey` true _asbp_first_person_character)
  (set `/Game/FirstPerson/Blueprints/BP_FirstPersonCharacter.CurrentKey` null _asbp_first_person_character)
  (`self.SetActorHiddenInGame` (`self.HallwayDoll`) true)
  (`self.SetActorHiddenInGame` (`self.ScareDoll`) false)
  (`GameplayStatics.PlaySoundAtLocation` "/Game/freesound_community-075283_quotbehind-youquot-whisper-86744.freesound_community-075283_quotbehind-youquot-whisper-86744" (`self.K2_GetActorLocation` _asbp_first_person_character) (struct) 1.0 1.0 0.0 null null null null)
  (bind _returnvalue (`|CreateWidget` "/Game/LevelPrototyping/WBP_KeyFound.WBP_KeyFound_C" (`GameplayStatics.GetPlayerController` 0)))
  (set `self.KeyFoundWidget` _returnvalue)
  (`UserWidget.AddToViewport` _returnvalue 0)
  (`KismetSystemLibrary.Delay` 1.0)
  (`Widget.RemoveFromParent` (`self.KeyFoundWidget`))
  (`self.K2_DestroyActor`))

(fn `UserConstructionScript`)