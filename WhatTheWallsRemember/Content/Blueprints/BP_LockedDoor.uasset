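; Key-locked door that swings open for the first-person player and triggers a BP_ShadowFigure crossing as a scare.
; InteractCollision overlaps set the player's CurrentDoor and toggle the interact prompt.
; Interact checks the player's HasKey, then plays a timeline that rotates DoorMesh, or shows a locked message if still closed.
; Each timeline update also spawns a new shadow figure moving between two reference actors, with no once-only guard.
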(event `self.ReceiveActorBeginOverlap`
  (params (OtherActor :type "Actor Object Reference"))
  (if true
    _))

(event `self.InteractCollision.OnComponentBeginOverlap`
  (params (OverlappedComponent :type "PrimitiveComponent Object Reference") (OtherActor :type "Actor Object Reference") (OtherComp :type "PrimitiveComponent Object Reference") (OtherBodyIndex :type Integer) (bFromSweep :type Boolean) (SweepResult :type "HitResult Structure (by ref)"))
  (bind _asbp_first_person_character (cast `/Game/FirstPerson/Blueprints/BP_FirstPersonCharacter` OtherActor))
  (set `self.PlayerInRange` true)
  (set `/Game/FirstPerson/Blueprints/BP_FirstPersonCharacter.CurrentDoor` self _asbp_first_person_character)
  (`/Game/FirstPerson/Blueprints/BP_FirstPersonCharacter.ShowInteractPrompt` _asbp_first_person_character))

(event `self.InteractCollision.OnComponentEndOverlap`
  (params (OverlappedComponent :type "PrimitiveComponent Object Reference") (OtherActor :type "Actor Object Reference") (OtherComp :type "PrimitiveComponent Object Reference") (OtherBodyIndex :type Integer))
  (bind _asbp_first_person_character (cast `/Game/FirstPerson/Blueprints/BP_FirstPersonCharacter` OtherActor))
  (set `self.PlayerInRange` false)
  (set `/Game/FirstPerson/Blueprints/BP_FirstPersonCharacter.CurrentDoor` null _asbp_first_person_character)
  (`/Game/FirstPerson/Blueprints/BP_FirstPersonCharacter.HideInteractPrompt` _asbp_first_person_character))

(event `Interact`
  (bind _asbp_first_person_character (cast `/Game/FirstPerson/Blueprints/BP_FirstPersonCharacter` (`GameplayStatics.GetPlayerCharacter` 0)))
  (if (`/Game/FirstPerson/Blueprints/BP_FirstPersonCharacter.HasKey` _asbp_first_person_character)
    (set `self.bDoorOpened` true)
    (bind (_direction _doorrotation) (`Timeline|TL_OpenDoor`)
      (:`Update`
        (`SceneComponent.K2_SetRelativeRotation` (`self.DoorMesh`) (`KismetMathLibrary.MakeRotator` 0.0 0.0 _doorrotation) false false)
        (if true
          (bind _returnvalue (`|SpawnActorFromClass` "/Game/Whisper/BP_ShadowFigure.BP_ShadowFigure_C" (`KismetMathLibrary.MakeTransform` (`self.K2_GetActorLocation` (`self.ShadowStartRef`))) "Undefined" "MultiplyWithRoot" null null))
          (set `/Game/Whisper/BP_ShadowFigure.StartLocation` (`self.K2_GetActorLocation` (`self.ShadowStartRef`)) _returnvalue)
          (set `/Game/Whisper/BP_ShadowFigure.EndLocation` (`self.K2_GetActorLocation` (`self.ShadowEndRef`)) _returnvalue)
          (`/Game/Whisper/BP_ShadowFigure.StartShadowCross` _returnvalue))))
    (elif (not (`self.bDoorOpened`))
      (bind _asbp_first_person_character_2 (cast `/Game/FirstPerson/Blueprints/BP_FirstPersonCharacter` (`GameplayStatics.GetPlayerCharacter` 0)))
      (`/Game/FirstPerson/Blueprints/BP_FirstPersonCharacter.ShowDoorLockedMessage` _asbp_first_person_character_2))))

(fn `UserConstructionScript`)