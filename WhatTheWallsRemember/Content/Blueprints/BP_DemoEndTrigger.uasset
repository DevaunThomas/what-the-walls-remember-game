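; Trigger actor that plays the demo's ending when the first-person player character enters its EndTrigger volume.
; A one-shot flag guards the overlap, which reveals the hidden ShadowActor and plays an end sting at the player's location.
; After a short delay, it creates the demo-end widget for the first player controller and adds it to the viewport.
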(event `self.EndTrigger.OnComponentBeginOverlap`
  (params (OverlappedComponent :type "PrimitiveComponent Object Reference") (OtherActor :type "Actor Object Reference") (OtherComp :type "PrimitiveComponent Object Reference") (OtherBodyIndex :type Integer) (bFromSweep :type Boolean) (SweepResult :type "HitResult Structure (by ref)"))
  (bind _asbp_first_person_character (cast `/Game/FirstPerson/Blueprints/BP_FirstPersonCharacter` OtherActor))
  (if (not (`self.HasTriggered`))
    (set `self.HasTriggered` true)
    (`self.SetActorHiddenInGame` (`self.ShadowActor`) false)
    (`GameplayStatics.PlaySoundAtLocation` (`self.EndSting`) (`self.K2_GetActorLocation` _asbp_first_person_character) (struct) 1.0 1.0 0.0 null null null null)
    (`KismetSystemLibrary.Delay` 1.0)
    (bind _returnvalue (`|CreateWidget` "/Game/LevelPrototyping/WBP_DemoEnd.WBP_DemoEnd_C" (`GameplayStatics.GetPlayerController` 0)))
    (`UserWidget.AddToViewport` _returnvalue 0)))

(fn `UserConstructionScript`)