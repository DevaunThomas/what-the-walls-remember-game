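; Game player controller that toggles a pause menu when P is pressed.
; If unpaused, it creates and shows a new WBP_PauseMenu, pauses the game, shows the cursor with click events enabled, and switches to UI-only input focused on the menu.
; If paused, it removes the widget, unpauses, hides the cursor, and restores game-only input.
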(event `Key|P`
  (params (Key :type "Key Structure"))
  (:`Pressed`
    (`KismetSystemLibrary.PrintString` "PAUSE PRESSED")
    (if (`GameplayStatics.IsGamePaused`)
      (`Widget.RemoveFromParent` (stale _returnvalue))
      (`GameplayStatics.SetGamePaused` false)
      (set `self.bShowMouseCursor` false)
      (`WidgetBlueprintLibrary.SetInputMode_GameOnly` null)
      (else
        (bind _returnvalue (`|CreateWidget` "/Game/WBP_PauseMenu.WBP_PauseMenu_C"))
        (bind _output_get (set `self.PauseMenuWidget` _returnvalue))
        (`UserWidget.AddToViewport` _output_get 0)
        (`GameplayStatics.SetGamePaused` true)
        (set `self.bShowMouseCursor` true)
        (`WidgetBlueprintLibrary.SetInputMode_UIOnlyEx` null _returnvalue)
        (set `self.bEnableClickEvents` true)))))

(fn `UserConstructionScript`)