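; BP_AIDirector is a horror director that plays timed ghost whispers and periodically reacts to the player's behavior type.
; BeginPlay schedules three 2D whispers and loops EvaluateTension, which reads PlayerType from BP_HouseMemoryManager to set tension gain and cooldown.
; Each evaluation accumulates Tension, and recognized types trigger a delay-chained visibility flicker on FlickerLightRef and the director's own root.
; The cooldown-gated house event is unfinished: its logic is disconnected and TriggerHouseEvent is empty.
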(event `TriggerLightFlicker`
  (bind _flickerlightref (`self.FlickerLightRef`))
  (`SceneComponent.SetVisibility` (`Light.LightComponent` _flickerlightref) false false)
  (`KismetSystemLibrary.Delay` 0.1)
  (`SceneComponent.SetVisibility` (`Actor.RootComponent` _flickerlightref) true false)
  (`KismetSystemLibrary.Delay` 0.1)
  (`SceneComponent.SetVisibility` (`Actor.RootComponent` _flickerlightref) false false)
  (`KismetSystemLibrary.Delay` 0.1)
  (`SceneComponent.SetVisibility` (`Actor.RootComponent` _flickerlightref) true false)
  (`KismetSystemLibrary.Delay` 0.1)
  (`SceneComponent.SetVisibility` (`self.RootComponent`) false false)
  (`KismetSystemLibrary.Delay` 0.1)
  (`SceneComponent.SetVisibility` (`self.RootComponent`) true false))

(event `TriggerHouseEvent`)

(event `self.ReceiveBeginPlay`
  (`KismetSystemLibrary.K2_SetTimerDelegate` (delegate `EvaluateTension`) 25.0 true)
  (`KismetSystemLibrary.Delay` 10.0)
  (`GameplayStatics.SpawnSound2D` "/Game/fadingembersaudio-creepy-female-ghost-whispers-430175.fadingembersaudio-creepy-female-ghost-whispers-430175" 1.0 1.0 0.0 null)
  (`KismetSystemLibrary.Delay` 15.0)
  (`GameplayStatics.SpawnSound2D` "/Game/Whispers_of_Macabre/dragon-studio-i-see-you-creepy-ghost-whisper-401711.dragon-studio-i-see-you-creepy-ghost-whisper-401711" 1.0 1.0 0.0 null)
  (`KismetSystemLibrary.Delay` 60.0)
  (`GameplayStatics.SpawnSound2D` "/Game/fadingembersaudio-creepy-female-ghost-whispers-430175.fadingembersaudio-creepy-female-ghost-whispers-430175" 1.0 1.0 0.0 null))

(event `EvaluateTension`
  (bind _outactors (`GameplayStatics.GetAllActorsOfClass` "/Game/BP_HouseMemoryManager.BP_HouseMemoryManager_C"))
  (bind _asbp_house_memory_manager (cast `/Game/BP_HouseMemoryManager` (`|GetArrayItem` _outactors)))
  (switch `string` (`/Game/BP_HouseMemoryManager.PlayerType` _asbp_house_memory_manager)
    (:`Default`
      (set `self.Tension` (+ (`self.Tension`) (`self.TensionGain`))))
    (:`Calm`
      (set `self.TensionGain` 0.5)
      (set `self.CurrentCooldown` 30.0)
      (set `self.Tension` (+ (`self.Tension`) (`self.TensionGain`)) :!label _label)
      (`self.TriggerLightFlicker`))
    (:`Cautious`
      (set `self.TensionGain` 1.0)
      (set `self.CurrentCooldown` 15.0)
      (goto _label))
    (:`Nervous`
      (set `self.TensionGain` 1.5)
      (set `self.CurrentCooldown` 7.0)
      (goto _label))
    (:`Panicked`
      (set `self.TensionGain` 2.0)
      (set `self.CurrentCooldown` 4.0)
      (goto _label))))

(fn `UserConstructionScript`)