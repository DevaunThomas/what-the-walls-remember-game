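; BP_DoorInteract is a door interaction actor that tracks player proximity through an InteractCollision component, with its interaction logic unfinished.
; Begin overlap sets PlayerInRange for any actor; end overlap clears it and the CurrentDoor reference on BP_FirstPersonCharacter.
; The logic that assigns itself as CurrentDoor is disconnected and never runs.
; The Interact event only casts the player character and performs no door action.
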(event `self.ReceiveActorBeginOverlap`
  (params (OtherActor :type "Actor Object Reference"))
  (if true
    _))

(event `self.InteractCollision.OnComponentBeginOverlap`
  (params (OverlappedComponent :type "PrimitiveComponent Object Reference") (OtherActor :type "Actor Object Reference") (OtherComp :type "PrimitiveComponent Object Reference") (OtherBodyIndex :type Integer) (bFromSweep :type Boolean) (SweepResult :type "HitResult Structure (by ref)"))
  (set `self.bPlayerInRange` true))

(event `Interact`
  (cast `/Game/FirstPerson/Blueprints/BP_FirstPersonCharacter` (`GameplayStatics.GetPlayerCharacter` 0)))

(event `self.InteractCollision.OnComponentEndOverlap`
  (params (OverlappedComponent :type "PrimitiveComponent Object Reference") (OtherActor :type "Actor Object Reference") (OtherComp :type "PrimitiveComponent Object Reference") (OtherBodyIndex :type Integer))
  (bind _asbp_first_person_character (cast `/Game/FirstPerson/Blueprints/BP_FirstPersonCharacter` OtherActor))
  (set `self.bPlayerInRange` false)
  (set `/Game/FirstPerson/Blueprints/BP_FirstPersonCharacter.CurrentDoor` null _asbp_first_person_character))

(fn `UserConstructionScript`)