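; BP_HouseMemoryManager is an actor that samples the player character's movement speed as a form of player memory.
; On BeginPlay it starts a looping quarter-second timer that reads the velocity magnitude of player character 0.
; Each tick of the timer averages that speed with the stored average, weighting recent samples heavily, and prints both values to screen for debugging.
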(event `self.ReceiveBeginPlay`
  (`KismetSystemLibrary.K2_SetTimerDelegate` (delegate `UpdatePlayerMemory`) 0.25 true))

(event `UpdatePlayerMemory`
  (set `self.PlayerSpeed` (`KismetMathLibrary.VSize` (`self.GetVelocity` (`GameplayStatics.GetPlayerCharacter` 0))))
  (set `self.PlayerSpeedAverage` (/ (+ (`self.PlayerSpeedAverage`) (`self.PlayerSpeed`)) 2.0))
  (`KismetSystemLibrary.PrintString` (`KismetStringLibrary.Concat_StrStr` "Speed: " (`KismetStringLibrary.Conv_DoubleToString` (`self.PlayerSpeed`))))
  (`KismetSystemLibrary.PrintString` (`KismetStringLibrary.Concat_StrStr` "Avg Speed: " (`KismetStringLibrary.Conv_DoubleToString` (`self.PlayerSpeedAverage`)))))

(fn `UserConstructionScript`)