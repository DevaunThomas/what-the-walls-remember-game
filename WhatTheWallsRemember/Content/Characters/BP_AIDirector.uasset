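; BP_AIDirector is a work-in-progress director meant to pace house events from a Tension value.
; On BeginPlay it starts a looping one-second timer on EvaluateTension, but that event is empty, so only debug prints run.
; Disconnected logic reads PlayerType from BP_HouseMemoryManager, adjusts Tension per player state, and calls TriggerHouseEvent behind a ForceTrue flag.
; TriggerHouseEvent itself only prints, and the random, cooldown and clamp nodes are unused.
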(event `TriggerHouseEvent`
  (`KismetSystemLibrary.PrintString` "HOUSE EVENT TRIGGERED"))

(event `self.ReceiveBeginPlay`
  (`KismetSystemLibrary.PrintString` "DIRECTOR ALIVE")
  (`KismetSystemLibrary.K2_SetTimerDelegate` (delegate `EvaluateTension`) 1.0 true)
  (`KismetSystemLibrary.PrintString` "Timer started"))

(event `EvaluateTension`)

(fn `UserConstructionScript`)